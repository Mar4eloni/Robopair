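; BP_Garbage is a garbage pile actor that the player clears by repeatedly pressing DestroyGarbage while nearby.
; Box overlap by a TopDownController enables input and opens a gate; ending overlap with GarbageMesh, a different component, reverses both.
; Each gated press lowers GarbageAmmount, setting GarbageRemoved at zero or below.
; GarbageRemoval destroys flagged actors; BeginPlay sets a looping timer, but its function name is unspecified.
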(event OnComponentBeginOverlap(Box)
  (params (OverlappedComponent :type Primitive%20Component%20Object%20Reference) (OtherActor :type Actor%20Object%20Reference) (OtherComp :type Primitive%20Component%20Object%20Reference) (OtherBodyIndex :type Integer) (bFromSweep :type Boolean) (SweepResult :type Hit%20Result%20Structure%20%28by%20ref%29))
  (Utilities|Casting|CastToTopDownController OtherActor)
  (Input|EnableInput (Game|GetPlayerController 0))
  (Utilities|FlowControl|Gate true) ; enters at Open
)

(event OnComponentEndOverlap(GarbageMesh)
  (params (OverlappedComponent :type Primitive%20Component%20Object%20Reference) (OtherActor :type Actor%20Object%20Reference) (OtherComp :type Primitive%20Component%20Object%20Reference) (OtherBodyIndex :type Integer))
  (Utilities|Casting|CastToTopDownController OtherActor)
  (Input|DisableInput (Game|GetPlayerController 0))
  (Utilities|FlowControl|Gate true) ; enters at Close
)

(event EventBeginPlay
  (Utilities|Time|SetTimerbyFunctionName 0 "" 0.6 true))

(event Collision|EventActorBeginOverlap
  (params (OtherActor :type Actor%20Object%20Reference)))

(event EventTick
  (params (DeltaSeconds :type Float%20%28single-precision%29)))

(event Input|ActionEvents|InputActionDestroyGarbage
  (params (Key :type Key%20Structure :default "None"))
  (:Pressed
    (Utilities|FlowControl|Gate true
      (:Exit
        (Variables|Default|SetGarbageAmmount (- (Variables|Default|GetGarbageAmmount) 25))
        (if (<= (Variables|Default|GetGarbageAmmount) 0)
          (Variables|Default|SetbGarbageRemoved true))))))

(fn ConstructionScript)

(fn GarbageRemoval
  (if (Variables|Default|GetbGarbageRemoved)
    (Actor|DestroyActor)))