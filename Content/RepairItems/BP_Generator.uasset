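; BP_Generator is a repairable generator that the player fixes with the repair items carried by the TopDownCharacter.
; Its Box overlap shows a hint, enables input and opens a gate for the Repair action.
; Repairing subtracts the character's RepairItems from ItemsNeeded, swaps meshes at thresholds and briefly pulses FinnishedRepairing on the character once the final mesh appears.
; A looping timer refreshes the remaining-parts text.
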(event OnComponentBeginOverlap(Box)
  (params (OverlappedComponent :type Primitive%20Component%20Object%20Reference) (OtherActor :type Actor%20Object%20Reference) (OtherComp :type Primitive%20Component%20Object%20Reference) (OtherBodyIndex :type Integer) (bFromSweep :type Boolean) (SweepResult :type Hit%20Result%20Structure%20%28by%20ref%29))
  (bind _astop_down_character (Utilities|Casting|CastToTopDownCharacter OtherActor))
  (Rendering|SetVisibility (Variables|Default|GetRepairHint) true false)
  (Input|EnableInput (Game|GetPlayerController 0))
  (Utilities|FlowControl|Gate true) ; enters at Open
)

(event OnComponentEndOverlap(Box)
  (params (OverlappedComponent :type Primitive%20Component%20Object%20Reference) (OtherActor :type Actor%20Object%20Reference) (OtherComp :type Primitive%20Component%20Object%20Reference) (OtherBodyIndex :type Integer))
  (Utilities|Casting|CastToTopDownCharacter OtherActor)
  (Rendering|SetVisibility (Variables|Default|GetRepairHint) false false)
  (Input|DisableInput (Game|GetPlayerController 0))
  (Utilities|FlowControl|Gate true) ; enters at Close
)

(event EventBeginPlay
  (Utilities|Time|SetTimerbyFunctionName 0 "UpdateRemainingPartsText" 0.2 true))

(event Collision|EventActorBeginOverlap
  (params (OtherActor :type Actor%20Object%20Reference)))

(event EventTick
  (params (DeltaSeconds :type Float%20%28single-precision%29)))

(event Input|ActionEvents|InputActionRepair
  (params (Key :type Key%20Structure :default "None"))
  (:Pressed
    (Audio|PlaySound2D "/Game/raboti_Cue.raboti_Cue" 1.0 1.0 0.0 0 0)
    (Utilities|FlowControl|Gate true
      (:Exit
        (if (<= (Variables|/Game/TopDownBP/Blueprints/TopDownCharacter.TopDownCharacter_C|GetRepairItems (stale OnComponentBeginOverlap(Box) _astop_down_character)) 0)
          (Development|PrintString "Not Enough Parts !")
          (elif (not (<= (Variables|Default|GetItemsNeeded) 0))
            (Variables|Default|SetItemsNeeded (- (Variables|Default|GetItemsNeeded) (Variables|/Game/TopDownBP/Blueprints/TopDownCharacter.TopDownCharacter_C|GetRepairItems (stale OnComponentBeginOverlap(Box) _astop_down_character))))
            (if (<= (Variables|Default|GetItemsNeeded) 50)
              (Components|StaticMesh|SetStaticMesh (Variables|Default|GetRepairMesh) "/Game/RepairItems/Meshes/Generator/Generator_HalfFixed/GeneratorHalfBroken.GeneratorHalfBroken")
              (if (<= (Variables|Default|GetItemsNeeded) 25)
                (Components|StaticMesh|SetStaticMesh (Variables|Default|GetRepairMesh) "/Game/RepairItems/Meshes/Generator/Generator_Repaired/Generator.Generator")
                (Variables|/Game/TopDownBP/Blueprints/TopDownCharacter.TopDownCharacter_C|SetFinnishedRepairing (stale OnComponentBeginOverlap(Box) _astop_down_character) true)
                (Utilities|FlowControl|Delay 1.0)
                (Variables|/Game/TopDownBP/Blueprints/TopDownCharacter.TopDownCharacter_C|SetFinnishedRepairing (stale OnComponentBeginOverlap(Box) _astop_down_character) false)))))))))

(fn ConstructionScript)

(fn UpdateRemainingPartsText
  (bind _itemsneeded (Variables|Default|GetItemsNeeded))
  (bind _remainingpartstext (Variables|Default|GetRemainingPartsText))
  (if (<= _itemsneeded 0)
    (Rendering|Components|TextRender|SetText _remainingpartstext (Utilities|Text|ToText(String) (Utilities|String|Append "Remaining Parts :" "0")))
    (else
      (Rendering|Components|TextRender|SetText _remainingpartstext (Utilities|Text|ToText(String) (Utilities|String|Append "Remaining Parts :" (Utilities|String|ToString(Integer) _itemsneeded)))))))